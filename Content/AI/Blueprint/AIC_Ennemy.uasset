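; Enemy AI controller that runs the enemy behavior tree and tracks the player through perception.
; On begin play it sets up the BB_Ennemy blackboard and starts BT_Ennemy.
; Perception updates for PFUnrealCharacter actors write the sensed actor to the PlayerRef key, or clear it when sensing fails, so the tree knows whether the player is detected.
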(event `self.ReceiveBeginPlay`
  (`self.UseBlackboard` "/Game/AI/Behavior/BB_Ennemy.BB_Ennemy")
  (`self.RunBehaviorTree` "/Game/AI/Behavior/BT_Ennemy.BT_Ennemy"))

(event `self.AIPerception.OnTargetPerceptionUpdated`
  (params (Actor :type "Actor Object Reference") (Stimulus :type "AIStimulus Structure"))
  (bind _returnvalue (`AIBlueprintHelperLibrary.GetBlackboard` null))
  ;[1 1 1] Check si il voit le joueur.
  (if (`KismetMathLibrary.ClassIsChildOf` (`GameplayStatics.GetObjectClass` Actor) "/Script/PFUnreal.PFUnrealCharacter")
    (if (`.bSuccessfullySensed` (break `AIStimulus` Stimulus))
      (`BlackboardComponent.SetValueAsObject` _returnvalue "PlayerRef" Actor)
      (else
        (`BlackboardComponent.SetValueAsObject` _returnvalue "PlayerRef" null)))))

(fn `UserConstructionScript`)